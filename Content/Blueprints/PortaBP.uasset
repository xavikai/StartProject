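; PortaBP is a door that swings open or closed while the first-person character's EstatAccio action flag is true.
; Tick polls that flag and plays or reverses a timeline based on OpenClose, which flips when the timeline finishes.
; The timeline's curve lerps the actor between RotacioInicial and RotacioFinal.
; A box overlap sets and clears ObrePorta, but this graph never reads it, so proximity does not gate the motion.
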(event OnComponentBeginOverlap(BoxCollisionArea)
  (params (OverlappedComponent :type Primitive%20Component%20Object%20Reference) (OtherActor :type Actor%20Object%20Reference) (OtherComp :type Primitive%20Component%20Object%20Reference) (OtherBodyIndex :type Integer) (bFromSweep :type Boolean) (SweepResult :type Hit%20Result%20Structure%20%28by%20ref%29))
  (Variables|Default|Setobre_porta true))

(event OnComponentEndOverlap(BoxCollisionArea)
  (params (OverlappedComponent :type Primitive%20Component%20Object%20Reference) (OtherActor :type Actor%20Object%20Reference) (OtherComp :type Primitive%20Component%20Object%20Reference) (OtherBodyIndex :type Integer))
  (Variables|Default|Setobre_porta false))

(event EventTick
  (params (DeltaSeconds :type Float%20%28single-precision%29))
  (bind _asfirst_person_character (Utilities|Casting|CastToFirstPersonCharacter (Game|GetPlayerCharacter 0)))
  (if (Variables|/Game/FirstPersonBP/Blueprints/FirstPersonCharacter.FirstPersonCharacter_C|GetestatAccio _asfirst_person_character)
    (if (Variables|Default|GetopenClose)
      (bind _funciomoviment (Timeline|Timeline_0 Reverse)
        (:Update
          (Transformation|SetActorRotation (Math|Rotator|Lerp(Rotator) (Variables|Default|GetrotacioInicial) (Variables|Default|GetrotacioFinal) _funciomoviment)))
        (:Finished
          (if (Variables|Default|GetopenClose)
            (Variables|Default|SetopenClose false)
            (else
              (Variables|Default|SetopenClose true)))))
      (else
        (Timeline|Timeline_0 Play)))))

(fn ConstructionScript)